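; BP_TelpoAttack is a boss attack actor that damages the player when an overlap occurs.
; On BeginPlay it copies TelpoDamage from the BP_Boss found in the level.
; Any actor overlap subtracts that value directly from Bpplayer's Health, without checking which actor overlapped.
; Forward movement by Speed and delta time is present but disconnected, and Tick is empty, so this graph never moves the actor.
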(event `self.ReceiveBeginPlay`
  (bind _returnvalue (`GameplayStatics.GetActorOfClass` "/Game/BossFile/BP_Boss.BP_Boss_C"))
  (set `self.Telpo Damage` (`/Game/BossFile/BP_Boss.TelpoDamage` _returnvalue)))

(event `self.ReceiveActorBeginOverlap`
  (params (OtherActor :type "Actor Object Reference"))
  (bind _returnvalue (`GameplayStatics.GetActorOfClass` "/Game/BPplayeractor/bp-player.bp-player_C"))
  (set `/Game/BPplayeractor/bp-player.health` (- (`/Game/BPplayeractor/bp-player.health` _returnvalue) (`self.Telpo Damage`)) _returnvalue))

(event `self.ReceiveTick`
  (params (DeltaSeconds :type "Float (single-precision)"))
  ;[1 1 1] P = P0 + GetActorForward * speed * deltaSeconds
)

(fn `UserConstructionScript`)