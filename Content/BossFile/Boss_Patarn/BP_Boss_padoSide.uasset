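; Side wave ("pado") attack of the boss that travels forward, damaging and shoving the player on contact.
; Tick sweeps it along its forward vector at Speed, while BeginPlay plays a fire sound toggled after a delay and reads PadoDamage from BP_Boss.
; Player overlap passes a DoOnce gate, so a single hit subtracts that damage from player Health and pushes the player along the wave's forward direction.
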(event `self.ReceiveBeginPlay`
  (`|ExecutionSequence`
    (:`then_0`
      (`/Engine/EditorBlueprintResources/StandardMacros.DoOnce` false
        (:`Completed`
          (bind _returnvalue (`GameplayStatics.SpawnSound2D` "/Game/StarterContent/Audio/Fire01.Fire01" 1.0 1.0 0.0 null))
          (`KismetSystemLibrary.Delay` 5.0)
          (`ActorComponent.ToggleActive` _returnvalue))))
    (:`then_1`
      (bind _returnvalue_2 (`GameplayStatics.GetActorOfClass` "/Game/BossFile/BP_Boss.BP_Boss_C"))
      (set `self.Pado Damage` (`/Game/BossFile/BP_Boss.PadoDamage` _returnvalue_2))
      (goto _label :!via `Reset`))))

(event `self.ReceiveTick`
  (params (DeltaSeconds :type "Float (single-precision)"))
  (`self.K2_SetActorLocation` (+ (`self.K2_GetActorLocation`) (* (* (`self.GetActorForwardVector`) (`self.speed`)) DeltaSeconds)) true))

(event `self.ReceiveActorBeginOverlap`
  (params (OtherActor :type "Actor Object Reference"))
  (cast `/Game/BPplayeractor/bp-player` OtherActor)
  (`/Engine/EditorBlueprintResources/StandardMacros.DoOnce` false :!label _label
    (:`Completed`
      (bind _returnvalue (`GameplayStatics.GetActorOfClass` "/Game/BPplayeractor/bp-player.bp-player_C"))
      (set `/Game/BPplayeractor/bp-player.health` (- (`/Game/BPplayeractor/bp-player.health` _returnvalue) (`self.Pado Damage`)) _returnvalue)
      (`/Engine/EditorBlueprintResources/StandardMacros.DoOnce` false
        (:`Completed`
          (bind _returnvalue_2 (`GameplayStatics.GetActorOfClass` "/Game/BPplayeractor/bp-player.bp-player_C"))
          (`self.K2_SetActorLocation` _returnvalue_2 (+ (* (`KismetMathLibrary.Normal` (`self.GetActorForwardVector`)) 100.0) (`self.K2_GetActorLocation` _returnvalue_2)) false false))))))

(fn `UserConstructionScript`)